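; BP_GlobalOrigin is a Blueprint that picks up IP address settings from a GlobalOriginData actor in the level.
; Its construction script finds all GlobalOriginData actors and, if any exist, stores the first as Data.
; It then sets both ServerAddress and ClientAddress from the same GetIpAddress call on Data, without checking that one was found.
; The event graph holds only empty placeholder events.
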(event EventBeginPlay)

(event Collision|EventActorBeginOverlap
  (params (OtherActor :type Actor%20Object%20Reference)))

(event EventTick
  (params (DeltaSeconds :type Float%20%28single-precision%29)))

(fn ConstructionScript
  (Utilities|FlowControl|Sequence
    (:then_0
      (bind _outactors (Actor|GetAllActorsOfClass "/Script/cataract_final.GlobalOriginData"))
      (if (> (Utilities|Array|Length _outactors) 0)
        (Variables|Default|SetData (Utilities|Array|Get(acopy) _outactors))))
    (:then_1
      (Utilities|FlowControl|Sequence
        (:then_0
          (Variables|Default|SetServerAddress (Class|GlobalOriginData|GetIpAddress (Variables|Default|GetData))))
        (:then_1
          (Variables|Default|SetClientAddress (Class|GlobalOriginData|GetIpAddress (Variables|Default|GetData))))))))