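; BP_ClearCornealIncision is a picking-object group, apparently for the clear corneal incision step of an eye procedure.
; On BeginPlay it caches BP_PickObjBase child actors and UI_ImageBase widgets from its scene components into arrays.
; It then plays the EyeFocusing2 widget's focus effect if PickingObj2's state matches the requested one.
; It also exposes functions to hide all effects and fetch a child by index.
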(event EventBeginPlay
  ;[1 1 1] Begin Event
  (CallFunction|SetChildObjArray)
  (CallFunction|BeginFocusingEffect "NewEnumerator0"))

(fn ConstructionScript)

(fn SetChildObjArray
  (Utilities|FlowControl|Sequence
    (:then_0
      (for _array_element (Actor|GetAllChildActors true)
        (bind _asbp_pick_obj_base (Utilities|Casting|CastToBP_PickObjBase _array_element))
        (Utilities|Array|Add (Variables|Default|GetBPArray) _asbp_pick_obj_base)))
    (:then_1
      (for _array_element_2 (Components|GetChildrenComponents (Variables|Default|GetScene) true)
        (bind _aswidget_component (Utilities|Casting|CastToWidgetComponent _array_element_2))
        (bind _asui_image_base (Utilities|Casting|CastToUI_ImageBase (UserInterface|GetUserWidgetObject _aswidget_component)))
        (Utilities|Array|Add (Variables|Default|GetUIArray) _asui_image_base)))))

(fn BeginFocusingEffect
  (params (StateOnly :type E_PickState%20Enum :default "NewEnumerator0"))
  (bind _asbp_pick_obj_base (Utilities|Casting|CastToBP_PickObjBase (Variables|/Script/Engine.ChildActorComponent|GetChildActor (Variables|Default|GetPickingObj2))))
  (if (Utilities|Enum|Equal(Enum) (Variables|/Game/1_Blueprint/BP_PickObjBase.BP_PickObjBase_C|GetState _asbp_pick_obj_base) StateOnly)
    (bind _asui_image_base (Utilities|Casting|CastToUI_ImageBase (UserInterface|GetUserWidgetObject (Variables|Default|GetEyeFocusing2))))
    (Default|PlayTotalFocusEffect _asui_image_base 1.0)))

(fn EndFocusingEffect
  (for _array_element (Variables|Default|GetUIArray)
    (Default|HideEffect _array_element)))

(fn GetChildObj
  (params (Index :type Integer))
  (if (< Index (Utilities|Array|Length (Variables|Default|GetBPArray)))
    (return (Utilities|Array|Get(acopy) (Variables|Default|GetBPArray) Index))
    (else
      (return 0))))