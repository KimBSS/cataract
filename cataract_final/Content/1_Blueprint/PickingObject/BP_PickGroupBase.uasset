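; Base actor for a group of pickable child objects that checks they are picked in a consistent direction.
; On BeginPlay it gathers BP_PickObjBase child actors and links their Prev/Next references by class.
; Each tick it detects newly changed objects, sets or checks Direction through neighbor links, and calls Reset on reversal or after brief loss of "CPoint" overlap.
; Reset, Succeed and Fail are empty here, with Reset's former logic left disconnected.
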(event OnComponentBeginOverlap(Collision)
  (params (OverlappedComponent :type Primitive%20Component%20Object%20Reference) (OtherActor :type Actor%20Object%20Reference) (OtherComp :type Primitive%20Component%20Object%20Reference) (OtherBodyIndex :type Integer) (bFromSweep :type Boolean) (SweepResult :type Hit%20Result%20Structure%20%28by%20ref%29))
  ;[1 1 1] Overlap Event
  (if (Utilities|String|Contains (Utilities|GetDisplayName OtherComp) "CPoint")
    (Variables|Default|SetTime 0.0)
    (Variables|Default|SetIsColliding true)))

(event OnComponentEndOverlap(Collision)
  (params (OverlappedComponent :type Primitive%20Component%20Object%20Reference) (OtherActor :type Actor%20Object%20Reference) (OtherComp :type Primitive%20Component%20Object%20Reference) (OtherBodyIndex :type Integer))
  ;[1 1 1] Overlap Event
  (if (Utilities|String|Contains (Utilities|GetDisplayName OtherComp) "CPoint")
    (Variables|Default|SetIsColliding false)))

(event EventBeginPlay
  ;[1 1 1] Begin Event
  (CallFunction|SetChildObjArray))

(event EventSucceed
  (params (CurrentObj :type BP%20Pick%20Obj%20Base%20Object%20Reference)))

(event EventFail
  (params (CurrentObj :type BP%20Pick%20Obj%20Base%20Object%20Reference)))

(event EventTick
  (params (DeltaSeconds :type Float%20%28single-precision%29))
  ;[1 1 1] Tick Event
  (CallFunction|CheckFlow)
  (if (not (Variables|Default|GetIsColliding))
    (if (> (Variables|Default|GetTime) 0.1)
      (CallFunction|Reset)
      (else
        (Variables|Default|SetTime (+ (Variables|Default|GetTime) (Utilities|Time|GetWorldDeltaSeconds)))))))

(fn ConstructionScript)

(fn SetChildObjArray
  (Utilities|FlowControl|Sequence
    (:then_0
      (for _array_element (Actor|GetAllChildActors true)
        (bind _asbp_pick_obj_base (Utilities|Casting|CastToBP_PickObjBase _array_element))
        (Utilities|Array|Add (Variables|Default|GetBPArray) _asbp_pick_obj_base)))
    (:then_1
      (for _array_element_2 (Variables|Default|GetBPArray)
        (LocalVariables|SetCurrent _array_element_2)
        (for _array_element_3 (Variables|Default|GetBPArray)
          (Utilities|FlowControl|Sequence
            (:then_0
              (if (== (Utilities|GetClass _array_element_3) (Variables|/Game/1_Blueprint/BP_PickObjBase.BP_PickObjBase_C|GetPrevClass (LocalVariables|GetCurrent)))
                (Variables|/Game/1_Blueprint/BP_PickObjBase.BP_PickObjBase_C|SetPrev (LocalVariables|GetCurrent) _array_element_3)))
            (:then_1
              (if (== (Utilities|GetClass _array_element_3) (Variables|/Game/1_Blueprint/BP_PickObjBase.BP_PickObjBase_C|GetNextClass (LocalVariables|GetCurrent)))
                (Variables|/Game/1_Blueprint/BP_PickObjBase.BP_PickObjBase_C|SetNext (LocalVariables|GetCurrent) _array_element_3)))))))))

(fn Reset)

(fn CheckFlow
  (Utilities|FlowControl|Sequence
    (:then_0
      (Utilities|Array|Clear (LocalVariables|GetSrcBPArray))
      (for _array_element (Variables|Default|GetBPArray)
        (if (Utilities|Enum|Equal(Enum) (Variables|/Game/1_Blueprint/BP_PickObjBase.BP_PickObjBase_C|GetState _array_element) "NewEnumerator3")
          (Utilities|Array|Add (LocalVariables|GetSrcBPArray) _array_element)))
      (LocalVariables|SetDstBPArray (LocalVariables|GetSrcBPArray))
      (for _array_element_2 (LocalVariables|GetSrcBPArray)
        (if (>= (Utilities|Array|FindItem (Variables|Default|GetS-BPArray) _array_element_2) 0)
          (Utilities|Array|RemoveItem (LocalVariables|GetDstBPArray) _array_element_2))))
    (:then_1
      (if (> (Utilities|Array|Length (LocalVariables|GetSrcBPArray)) 3)
        (if (> (Utilities|Array|Length (LocalVariables|GetDstBPArray)) 0)
          (bind _output_get (LocalVariables|SetNew (Utilities|Array|Get(acopy) (LocalVariables|GetDstBPArray))))
          (Utilities|IsValid _output_get
            (:Is%20Valid
              (for _array_element_3 (LocalVariables|GetSrcBPArray)
                (LocalVariables|SetCurrent _array_element_3)
                (if (CallFunction|CheckLinkageAND (LocalVariables|GetCurrent))
                  (if (== (Variables|Default|GetDirection) 0)
                    (if (== (Variables|/Game/1_Blueprint/BP_PickObjBase.BP_PickObjBase_C|GetPrev (LocalVariables|GetCurrent)) (LocalVariables|GetNew))
                      (Variables|Default|SetDirection -1)
                      (return)
                      (else
                        (Variables|Default|SetDirection 1)
                        (return)))
                    (elif (== (Variables|Default|GetDirection) 1)
                      (if (== (Variables|/Game/1_Blueprint/BP_PickObjBase.BP_PickObjBase_C|GetPrev (LocalVariables|GetCurrent)) (LocalVariables|GetNew))
                        (CallFunction|Reset)
                        (return))
                      (elif (== (Variables|/Game/1_Blueprint/BP_PickObjBase.BP_PickObjBase_C|GetNext (LocalVariables|GetCurrent)) (LocalVariables|GetNew))
                        (CallFunction|Reset)
                        (return)))))))))))
    (:then_3
      (Variables|Default|SetS-BPArray (LocalVariables|GetSrcBPArray)))))

(fn CheckLinkageOR
  (params (Current :type BP%20Pick%20Obj%20Base%20Object%20Reference))
  (if (and (Utilities|IsValid (Variables|/Game/1_Blueprint/BP_PickObjBase.BP_PickObjBase_C|GetPrev Current)) (Utilities|IsValid (Variables|/Game/1_Blueprint/BP_PickObjBase.BP_PickObjBase_C|GetNext Current)))
    (return (or (Utilities|Enum|Equal(Enum) (Variables|/Game/1_Blueprint/BP_PickObjBase.BP_PickObjBase_C|GetState (Variables|/Game/1_Blueprint/BP_PickObjBase.BP_PickObjBase_C|GetPrev Current)) "NewEnumerator3") (Utilities|Enum|Equal(Enum) (Variables|/Game/1_Blueprint/BP_PickObjBase.BP_PickObjBase_C|GetState (Variables|/Game/1_Blueprint/BP_PickObjBase.BP_PickObjBase_C|GetNext Current)) "NewEnumerator3")))
    (else
      (return false))))

(fn CheckLinkageAND
  (params (CurrentObj :type BP%20Pick%20Obj%20Base%20Object%20Reference))
  (if (and (Utilities|IsValid (Variables|/Game/1_Blueprint/BP_PickObjBase.BP_PickObjBase_C|GetPrev CurrentObj)) (Utilities|IsValid (Variables|/Game/1_Blueprint/BP_PickObjBase.BP_PickObjBase_C|GetNext CurrentObj)))
    (return (and (Utilities|Enum|Equal(Enum) (Variables|/Game/1_Blueprint/BP_PickObjBase.BP_PickObjBase_C|GetState (Variables|/Game/1_Blueprint/BP_PickObjBase.BP_PickObjBase_C|GetPrev CurrentObj)) "NewEnumerator3") (Utilities|Enum|Equal(Enum) (Variables|/Game/1_Blueprint/BP_PickObjBase.BP_PickObjBase_C|GetState (Variables|/Game/1_Blueprint/BP_PickObjBase.BP_PickObjBase_C|GetNext CurrentObj)) "NewEnumerator3")))
    (else
      (return false))))

(fn GetChildObj
  (params (Index :type Integer))
  (if (< Index (Utilities|Array|Length (Variables|Default|GetBPArray)))
    (return (Utilities|Array|Get(acopy) (Variables|Default|GetBPArray) Index))
    (else
      (return 0))))