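; BP_IOLinsertion is an actor in the PickingObject folder, apparently for intraocular lens insertion, that plays a lens insertion effect.
; Its InsertLensEffect event makes the Lens component visible and plays a timeline from the start.
; The timeline's Scale track drives the Lens relative X scale, with Y and Z held at one.
; BeginPlay, overlap and Tick are inactive placeholder nodes, and the construction script only calls the parent.
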(event Custom|InsertLensEffect
  ;[1 1 1] Insert Lens Effect Event
  (Rendering|SetVisibility (Variables|Default|GetLens) true false)
  (bind _scale (Timeline|타임라인_0 PlayFromStart)
    (:Update
      (Transformation|SetRelativeScale3D (Variables|Default|GetLens) (Math|Vector|MakeVector _scale 1.0 1.0)))))

(event EventBeginPlay
  (|CallParentFunction))

(event Collision|EventActorBeginOverlap
  (params (OtherActor :type Actor%20Object%20Reference)))

(event EventTick
  (params (DeltaSeconds :type Float%20%28single-precision%29))
  (|CallParentFunction DeltaSeconds))

(fn ConstructionScript
  (|CallParentFunction))