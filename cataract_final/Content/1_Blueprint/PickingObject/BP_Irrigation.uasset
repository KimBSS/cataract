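; BP_Irrigation is an irrigation picking-object Blueprint that displays an animated circle-arrow indicator.
; On BeginPlay it runs the parent logic, caches the CircleArrow widget component's UI_ImageBase as CircleArrowUI and starts that widget's total fade effect.
; Each tick it runs the parent logic, then spins the CircleArrow component around its roll axis at a constant, frame-rate-independent speed.
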(event EventBeginPlay
  ;[1 1 1] Begin Event
  (|CallParentFunction)
  (bind _asui_image_base (Utilities|Casting|CastToUI_ImageBase (UserInterface|GetUserWidgetObject (Variables|Default|GetCircleArrow))))
  (bind _output_get (Variables|Default|SetCircleArrowUI _asui_image_base))
  (Default|PlayTotalFadeEffect _output_get 0.5))

(event EventTick
  (params (DeltaSeconds :type Float%20%28single-precision%29))
  ;[1 1 1] Tick Event
  (|CallParentFunction DeltaSeconds)
  (Transformation|AddRelativeRotation (Variables|Default|GetCircleArrow) (Math|Rotator|MakeRotator (* (Utilities|Time|GetWorldDeltaSeconds) -1e+02) 0.0 0.0) false false))

(fn ConstructionScript
  (|CallParentFunction))