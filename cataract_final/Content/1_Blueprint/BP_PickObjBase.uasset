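; BP_PickObjBase is a pickable object that succeeds when a motion controller overlaps it long enough.
; Overlap begins picking and enables Tick, which accumulates the hold time and reports it to the OptiTrack player pawn until the success threshold.
; Leaving early resets progress as a failure, and both outcomes are reported to the parent actor.
; A dynamic material recolors the mesh blue while picking, green on success and red on failure.
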(event OnComponentBeginOverlap(ObjMesh)
  (params (OverlappedComponent :type Primitive%20Component%20Object%20Reference) (OtherActor :type Actor%20Object%20Reference) (OtherComp :type Primitive%20Component%20Object%20Reference) (OtherBodyIndex :type Integer) (bFromSweep :type Boolean) (SweepResult :type Hit%20Result%20Structure%20%28by%20ref%29))
  ;[1 1 1] Picking Event
  (Utilities|Casting|CastToBP_MotionController OtherActor)
  (CallFunction|BeginPicking)
  (Actor|Tick|SetActorTickEnabled true))

(event OnComponentEndOverlap(ObjMesh)
  (params (OverlappedComponent :type Primitive%20Component%20Object%20Reference) (OtherActor :type Actor%20Object%20Reference) (OtherComp :type Primitive%20Component%20Object%20Reference) (OtherBodyIndex :type Integer))
  ;[1 1 1] Picking Event
  (Utilities|Casting|CastToBP_MotionController OtherActor)
  (CallFunction|Fail false)
  (Actor|Tick|SetActorTickEnabled false))

(event EventBeginPlay
  ;[1 1 1] Begin Event
  (CallFunction|InitPlayerPawn)
  (CallFunction|InitMaterialInstance)
  (Actor|Tick|SetActorTickEnabled false))

(event EventTick
  (params (DeltaSeconds :type Float%20%28single-precision%29))
  ;[1 1 1] Tick Event
  (if (Utilities|Enum|Equal(Enum) (Variables|Default|GetState) "NewEnumerator2")
    (if (>= (Variables|Default|GetPickingTime) (Variables|Default|GetSuccessTme))
      (CallFunction|Succeed)
      (else
        (bind _output_get (Variables|Default|SetPickingTime (+ (Variables|Default|GetPickingTime) (Utilities|Time|GetWorldDeltaSeconds))))
        (Default|UpdatePickingTime (Variables|Default|GetPlayerPawn) _output_get)))))

(fn ConstructionScript)

(fn BeginPicking
  (if (Utilities|Enum|Equal(Enum) (Variables|Default|GetState) "NewEnumerator0")
    (Variables|Default|SetState "NewEnumerator2")
    (Default|BeginPickingTime (Variables|Default|GetPlayerPawn) self)
    (CallFunction|SetColor "(R=0.000000,G=0.000000,B=1.000000,A=1.000000)")))

(fn Fail
  (params (Force :type Boolean))
  (if (or (Utilities|Enum|Equal(Enum) (Variables|Default|GetState) "NewEnumerator2") Force)
    (Variables|Default|SetState "NewEnumerator0")
    (Variables|Default|SetPickingTime 0.0)
    (Default|ResetPickingTime (Variables|Default|GetPlayerPawn))
    (CallFunction|SetColor "(R=1.000000,G=0.000000,B=0.000000,A=1.000000)")
    (Class|BIPickingObj|Fail(Message) (Actor|GetParentActor) self)))

(fn Succeed
  (Variables|Default|SetState "NewEnumerator3")
  (Default|ResetPickingTime (Variables|Default|GetPlayerPawn))
  (CallFunction|SetColor "(R=0.000000,G=1.000000,B=0.000000,A=1.000000)")
  (Class|BIPickingObj|Succeed(Message) (Actor|GetParentActor) self))

(fn InitMaterialInstance
  (bind _returnvalue (Rendering|Material|CreateDynamicMaterialInstance (Variables|Default|GetObjMesh) 0 0 :!class /Script/Engine.PrimitiveComponent))
  (Variables|Default|SetMaterialInstance _returnvalue))

(fn InitPlayerPawn
  (bind _asbp_optitrack_player (Utilities|Casting|CastToBP_OptitrackPlayer (Game|Player|GetPlayerPawn 0)))
  (Variables|Default|SetPlayerPawn _asbp_optitrack_player))

(fn SetColor
  (params (Color :type Linear%20Color%20Structure))
  (Utilities|IsValid (Variables|Default|GetMaterialInstance)
    (:Is%20Valid
      (Rendering|Material|SetVectorParameterValue (Variables|Default|GetMaterialInstance) "Color" Color :!class /Script/Engine.MaterialInstanceDynamic))))