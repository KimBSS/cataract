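; BP_Face is a face actor that carries a spawned BP_Eye and a 2D scene capture restricted to registered actors.
; On BeginPlay it adds itself to the capture's show-only list, then spawns and attaches the eye, whose visibility follows the face's.
; Magnification either scales the eye actor or, in the render-target variant, enables per-frame capture and adjusts orthographic width.
; Getters expose the eye, its location and a reversed-rotation capture transform.
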(event EventBeginPlay
  ;[1 1 1] Begin Event
  (|CallParentFunction)
  (CallFunction|AddtoSceneCapture self)
  (bind _returnvalue (Game|SpawnActorfromClass "/Game/1_Blueprint/Eye/BP_Eye.BP_Eye_C" (Math|Transform|MakeTransform "0, 0, 0" "0, 0,-90.000000") "Undefined" 0 (Variables|Default|GetOnView) 0))
  (Transformation|AttachComponentToComponent _returnvalue (Variables|Default|GetDefaultSceneRoot) "None" "KeepRelative" "KeepRelative" "KeepRelative" true)
  (Variables|Default|SetEyeObject _returnvalue))

(event EventSetMeshVisible
  (params (Visible :type Boolean))
  ;[1 1 1] Set Mesh Visible
  (|CallParentFunction Visible)
  (Rendering|SetVisibility (Variables|/Game/1_Blueprint/Eye/BP_Eye.BP_Eye_C|GetRoot (Variables|Default|GetEyeObject)) Visible true))

(fn ConstructionScript
  (|CallParentFunction))

(fn GetReverseSceneCaptureTrans
  (bind _scenecapturecomponent2d (Variables|Default|GetSceneCaptureComponent2D))
  (return (Math|Transform|MakeTransform (Transformation|GetWorldLocation _scenecapturecomponent2d) (Class|KismetMathLibrary|NegateRotator (Transformation|GetWorldRotation _scenecapturecomponent2d)))))

(fn AddtoSceneCapture
  (params (Actor :type Actor%20Object%20Reference))
  (Utilities|Array|Add (Variables|/Script/Engine.SceneCaptureComponent|GetShowOnlyActors (Variables|Default|GetSceneCaptureComponent2D)) Actor))

(fn SetMagnificationRT
  (params (Magnfication :type Float%20%28single-precision%29))
  (Utilities|FlowControl|Sequence
    (:then_0
      (Variables|/Script/Engine.SceneCaptureComponent|SetbCaptureEveryFrame (Variables|Default|GetSceneCaptureComponent2D) true))
    (:then_1
      (Variables|/Script/Engine.SceneCaptureComponent2D|SetOrthoWidth (Variables|Default|GetSceneCaptureComponent2D) (Math|Float|Lerp 64.0 4.0 (/ 1e+01 Magnfication))))))

(fn SetMagnification
  (params (Magnification :type Float%20%28single-precision%29))
  (bind _returnvalue (/ Magnification 2e+01))
  (Transformation|SetActorScale3D (Variables|Default|GetEyeObject) (Math|Vector|MakeVector _returnvalue _returnvalue _returnvalue)))

(fn GetEyeObject
  (return (Variables|Default|GetEyeObject)))

(fn GetEyeLocation
  (Utilities|IsValid (Variables|Default|GetEyeObject)
    (:Is%20Valid
      (return (Transformation|GetActorLocation (Variables|Default|GetEyeObject))))
    (:Is%20Not%20Valid
      (return "0, 0, 0"))))