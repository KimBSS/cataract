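; BP_HandBase is a base Blueprint for a VR motion hand, extending parent logic for startup and mesh visibility.
; On BeginPlay it mirrors ObjectMesh along X for the left hand, and SetMeshVisible also toggles HandMesh without propagating to children.
; Helper functions activate, deactivate or destroy particle systems under the Point component, found by name substring through FindParticleSystem.
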(event EventBeginPlay
  ;[1 1 1] Begin Event
  (|CallParentFunction)
  (if (Utilities|Enum|Equal(Enum) (Variables|Default|GetHand) "Left")
    (Transformation|SetWorldScale3D (Variables|Default|GetObjectMesh) (* (Transformation|GetWorldScale (Variables|Default|GetObjectMesh)) "-1.000000,1.000000,1.000000"))))

(event EventTick
  (params (DeltaSeconds :type Float%20%28single-precision%29))
  (|CallParentFunction DeltaSeconds))

(event EventSetMeshVisible
  (params (Visible :type Boolean))
  ;[1 1 1] Set Mesh Visible
  (|CallParentFunction Visible)
  (Rendering|SetVisibility (Variables|Default|GetHandMesh) Visible false))

(fn ConstructionScript
  (|CallParentFunction))

(fn KillParticleSystem
  (params (SubName :type String))
  (bind _particlesystem (CallFunction|FindParticleSystem SubName))
  (Utilities|IsValid _particlesystem
    (:Is%20Valid
      (Components|DestroyComponent _particlesystem))))

(fn ActivateParticleSystem
  (params (SubName :type String))
  (bind _particlesystem (CallFunction|FindParticleSystem SubName))
  (Utilities|IsValid _particlesystem
    (:Is%20Valid
      (Components|Activation|Activate _particlesystem true))))

(fn FindParticleSystem
  (params (SubName :type String))
  (for _array_element (Components|GetChildrenComponents (Variables|Default|GetPoint) true)
    (bind _asparticle_system_component (Utilities|Casting|CastToParticleSystemComponent _array_element))
    (if (Utilities|String|Contains (Utilities|GetObjectName _asparticle_system_component) SubName)
      (return _asparticle_system_component)))
  (return 0))

(fn DeactivateParticleSystem
  (params (SubName :type String))
  (bind _particlesystem (CallFunction|FindParticleSystem SubName))
  (Utilities|IsValid _particlesystem
    (:Is%20Valid
      (Components|Activation|Deactivate _particlesystem))))