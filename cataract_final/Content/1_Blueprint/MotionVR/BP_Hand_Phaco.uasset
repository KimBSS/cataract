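; BP_Hand_Phaco is a MotionVR hand Blueprint, named for a phaco tool, that makes sure its particle effects start switched off.
; On BeginPlay it calls the parent logic, then DeactivateAllParticles walks all descendants of the Point component and deactivates the particle systems among them.
; The construction script only calls its parent, and Tick is disabled, so any other behavior comes from the parent class.
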(event EventBeginPlay
  ;[1 1 1] Begin Event
  (|CallParentFunction)
  (CallFunction|DeactivateAllParticles))

(event EventTick
  (params (DeltaSeconds :type Float%20%28single-precision%29))
  (|CallParentFunction DeltaSeconds))

(fn ConstructionScript
  (|CallParentFunction))

(fn DeactivateAllParticles
  (for _array_element (Components|GetChildrenComponents (Variables|Default|GetPoint) true)
    (bind _asparticle_system_component (Utilities|Casting|CastToParticleSystemComponent _array_element))
    (Components|Activation|Deactivate _asparticle_system_component)))