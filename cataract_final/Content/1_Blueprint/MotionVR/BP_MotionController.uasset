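; BP_MotionController is a motion-tracked VR object Blueprint driven by an OptiTrack rigid body component.
; On BeginPlay it passes its StreamingID to SetTrackingID, which sets the rigid body's TrackingId.
; SetMeshVisible shows or hides ObjectMesh and StaticMesh together, without propagating the change to their children.
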(event EventBeginPlay
  ;[1 1 1] Begin Event
  (CallFunction|SetTrackingID (Variables|Default|GetStreamingID)))

(fn ConstructionScript)

(fn SetTrackingID
  (params (Id :type Integer))
  (Variables|/Script/OptitrackNatnet.OptitrackRigidBodyComponent|SetTrackingId (Variables|Default|GetOptitrackRigidBody) Id))

(fn SetMeshVisible
  (params (Visible :type Boolean))
  (Utilities|FlowControl|Sequence
    (:then_0
      (Rendering|SetVisibility (Variables|Default|GetObjectMesh) Visible false))
    (:then_1
      (Rendering|SetVisibility (Variables|Default|GetStaticMesh) Visible false))))