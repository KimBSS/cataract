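; BP_Eye is the eye actor for what appears to be a VR eye-surgery procedure with a perfusion step.
; It line-traces the lens mesh to measure hand depth, feeds that to a UI_PerfusionGrid widget, and accumulates perfusion time while depth stays mid-range.
; It also swaps the divided lens for a capsule plus an attached detailed lens actor.
; The controller-overlap fail event has no effect; its failure message call is disconnected.
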(event OnComponentBeginOverlap(Cube)
  (params (OverlappedComponent :type Primitive%20Component%20Object%20Reference) (OtherActor :type Actor%20Object%20Reference) (OtherComp :type Primitive%20Component%20Object%20Reference) (OtherBodyIndex :type Integer) (bFromSweep :type Boolean) (SweepResult :type Hit%20Result%20Structure%20%28by%20ref%29))
  ;[1 1 1] Fail Event
  (Utilities|Casting|CastToBP_MotionController OtherActor)
  (if (Variables|Default|GetIsPerfusing)
    _))

(event EventTick
  (params (DeltaSeconds :type Float%20%28single-precision%29))
  ;[1 1 1] Tick Event
  (if (Variables|Default|GetIsPerfusing)
    (bind _succeed (CallFunction|IsProperDepthRange))
    (if _succeed
      (Variables|Default|SetPerfusingTime (+ (Variables|Default|GetPerfusingTime) (Utilities|Time|GetWorldDeltaSeconds))))
    (else
      (Variables|Default|SetPerfusingTime 0.0))))

(fn ConstructionScript)

(fn GetLensSurfacePosition
  (params (Input :type Vector) (Magnification :type Float%20%28single-precision%29))
  (bind (_x _y) (Math|Vector|BreakVector Input))
  (bind _returnvalue (Transformation|GetActorLocation))
  (bind _returnvalue_2 (Transformation|GetActorRotation))
  (LocalVariables|Sethalf_size (* (* (.X (Math|Vector|BreakVector (Transformation|GetActorScale3D))) 0.5) (Variables|Default|GetEyeLensRatio)))
  (LocalVariables|Setpos_x (* (* _x (LocalVariables|Gethalf_size)) Magnification))
  (LocalVariables|Setpos_z (* (* _y (LocalVariables|Gethalf_size)) Magnification))
  (bind (_hitlocation _hitnormal _bonename _outhit _returnvalue_3) (Collision|LineTraceComponent (Variables|Default|GetEyes_Divide_Lens) (+ (Math|Vector|RotateVector (Math|Vector|MakeVector (LocalVariables|Getpos_x) 1e+02 (LocalVariables|Getpos_z)) _returnvalue_2) _returnvalue) (+ (Math|Vector|RotateVector (Math|Vector|MakeVector (LocalVariables|Getpos_x) -1e+02 (LocalVariables|Getpos_z)) _returnvalue_2) _returnvalue) true false))
  (if _returnvalue_3
    (return _hitlocation)))

(fn GetCenterPos
  (return (Transformation|GetWorldLocation (Variables|Default|GetCenter))))

(fn GetPerfusingTime
  (return (Variables|Default|GetPerfusingTime)))

(fn SetPerfusingTime
  (params (Time :type Float%20%28single-precision%29))
  (Variables|Default|SetPerfusingTime Time))

(fn GetEyeTransform
  (bind _eyes_180510_3_eye (Variables|Default|GetEyes_180510_3_Eye))
  (return (Transformation|GetWorldLocation _eyes_180510_3_eye) (Transformation|GetWorldRotation _eyes_180510_3_eye)))

(fn SpawnEyeLensDetail
  (Rendering|SetVisibility (Variables|Default|GetEyes_Divide_Lens) false false)
  (Rendering|SetVisibility (Variables|Default|GetEyes_180510_3_Lens_Capsule) true false)
  (bind _returnvalue (Game|SpawnActorfromClass "/Game/1_Blueprint/Eye/BP_Eyes_Lens_Detail.BP_Eyes_Lens_Detail_C" (Math|Transform|MakeTransform "0,25.000000, 0") "Undefined" 0 0))
  (Transformation|AttachComponentToComponent _returnvalue (Variables|Default|GetRoot) "None" "KeepRelative" "KeepRelative" "KeepRelative" true)
  (Rendering|SetVisibility (Variables|Default|GetEyes_Divide_Lens) false false)
  (return _returnvalue))

(fn SetPerfusionDepth
  (params (HandPos :type Vector))
  (bind _result (CallFunction|GetLensSurfacePosition HandPos 1.0))
  (Variables|Default|SetDepth (Math|Vector|VectorLength (- HandPos _result)))
  (bind _asui_perfusion_grid (Utilities|Casting|CastToUI_PerfusionGrid (UserInterface|GetUserWidgetObject (Variables|Default|GetDepthGrid))))
  (Default|SetPivot _asui_perfusion_grid (/ (Variables|Default|GetDepth) (Variables|Default|GetMaxLensDistance))))

(fn BeginPerfusion
  (Rendering|SetVisibility (Variables|Default|GetDepthGrid) true false)
  (Variables|Default|SetIsPerfusing true))

(fn EndPerfusion
  (Rendering|SetVisibility (Variables|Default|GetDepthGrid) false false)
  (Variables|Default|SetIsPerfusing false))

(fn IsProperDepthRange
  (if (>= (Variables|Default|GetDepth) (* (Variables|Default|GetMaxLensDistance) 0.35))
    (if (<= (Variables|Default|GetDepth) (* (Variables|Default|GetMaxLensDistance) 0.65))
      (return true)
      (else
        (return false)))
    (else
      (return false))))