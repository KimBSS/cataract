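; Detailed eye lens actor for a VR phacoemulsification cataract surgery trainer, staging sculpting, nucleus rotation, cracking and quadrant removal by PhacoStep.
; Tool overlaps on box rows slice procedural nucleus meshes, while hand vectors around the center rotate the nucleus to a target angle.
; Timelines animate guide arrows, cracking and quadrant highlights; touched quadrants shatter as destructibles and scale through a timeline.
; Rotation, cracking and removal report completion to BP_OptitrackPlayer.
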(event OnComponentBeginOverlap(VerticalRegion)
  (params (OverlappedComponent :type Primitive%20Component%20Object%20Reference) (OtherActor :type Actor%20Object%20Reference) (OtherComp :type Primitive%20Component%20Object%20Reference) (OtherBodyIndex :type Integer) (bFromSweep :type Boolean) (SweepResult :type Hit%20Result%20Structure%20%28by%20ref%29))
  ;[1 1 1] Vertical Region Event
  (bind _asbp_hand_base (Utilities|Casting|CastToBP_HandBase OtherActor))
  (Variables|Default|SetHand_Phaco _asbp_hand_base)
  (if (Utilities|Enum|Equal(Enum) (Variables|Default|GetPhacoStep) "NewEnumerator13")
    (Variables|Default|SetEnteredVerticalRegion true)
    (bind _result (CallFunction|CalculateVector))
    (Variables|Default|SetVector0 _result)))

(event OnComponentEndOverlap(VerticalRegion)
  (params (OverlappedComponent :type Primitive%20Component%20Object%20Reference) (OtherActor :type Actor%20Object%20Reference) (OtherComp :type Primitive%20Component%20Object%20Reference) (OtherBodyIndex :type Integer))
  ;[1 1 1] Vertical Region Event
  (Utilities|Casting|CastToBP_HandBase OtherActor)
  (Variables|Default|SetHand_Phaco 0)
  (if (Utilities|Enum|Equal(Enum) (Variables|Default|GetPhacoStep) "NewEnumerator13")
    (Variables|Default|SetEnteredVerticalRegion false)))

(event OnComponentBeginOverlap(Eyes_180510_3_Lens_Nucleus_01)
  (params (OverlappedComponent :type Primitive%20Component%20Object%20Reference) (OtherActor :type Actor%20Object%20Reference) (OtherComp :type Primitive%20Component%20Object%20Reference) (OtherBodyIndex :type Integer) (bFromSweep :type Boolean) (SweepResult :type Hit%20Result%20Structure%20%28by%20ref%29))
  ;[1 1 1] Nucleus Remove
  (Utilities|Casting|CastToBP_Hand_Phaco OtherActor)
  (Utilities|FlowControl|Delay 0.5)
  (if (Utilities|Enum|Equal(Enum) (Variables|/Game/1_Blueprint/Player/BP_OptitrackPlayer.BP_OptitrackPlayer_C|GetPhacoStage (Variables|Default|GetPlayerPawn)) "NewEnumerator3")
    (CallFunction|DemolishNucleus (Variables|Default|GetEyes_180510_3_Lens_Nucleus_01) (Variables|Default|GetEyes_Lens_Nucleus_01_DM))))

(event OnComponentBeginOverlap(Eyes_180510_3_Lens_Nucleus_02)
  (params (OverlappedComponent :type Primitive%20Component%20Object%20Reference) (OtherActor :type Actor%20Object%20Reference) (OtherComp :type Primitive%20Component%20Object%20Reference) (OtherBodyIndex :type Integer) (bFromSweep :type Boolean) (SweepResult :type Hit%20Result%20Structure%20%28by%20ref%29))
  ;[1 1 1] Nucleus Remove
  (Utilities|Casting|CastToBP_Hand_Phaco OtherActor)
  (Utilities|FlowControl|Delay 0.5)
  (if (Utilities|Enum|Equal(Enum) (Variables|/Game/1_Blueprint/Player/BP_OptitrackPlayer.BP_OptitrackPlayer_C|GetPhacoStage (Variables|Default|GetPlayerPawn)) "NewEnumerator3")
    (CallFunction|DemolishNucleus (Variables|Default|GetEyes_180510_3_Lens_Nucleus_02) (Variables|Default|GetEyes_Lens_Nucleus_02_DM))))

(event OnComponentBeginOverlap(Eye_Lens)
  (params (OverlappedComponent :type Primitive%20Component%20Object%20Reference) (OtherActor :type Actor%20Object%20Reference) (OtherComp :type Primitive%20Component%20Object%20Reference) (OtherBodyIndex :type Integer) (bFromSweep :type Boolean) (SweepResult :type Hit%20Result%20Structure%20%28by%20ref%29))
  ;[1 1 1] Lens Region Event
  (Utilities|Casting|CastToBP_Hand_Phaco OtherActor)
  (Variables|Default|SetEnteredLensRegion true))

(event OnComponentBeginOverlap(Eyes_180510_3_Lens_Nucleus_03)
  (params (OverlappedComponent :type Primitive%20Component%20Object%20Reference) (OtherActor :type Actor%20Object%20Reference) (OtherComp :type Primitive%20Component%20Object%20Reference) (OtherBodyIndex :type Integer) (bFromSweep :type Boolean) (SweepResult :type Hit%20Result%20Structure%20%28by%20ref%29))
  ;[1 1 1] Nucleus Remove
  (Utilities|Casting|CastToBP_Hand_Phaco OtherActor)
  (Utilities|FlowControl|Delay 0.5)
  (if (Utilities|Enum|Equal(Enum) (Variables|/Game/1_Blueprint/Player/BP_OptitrackPlayer.BP_OptitrackPlayer_C|GetPhacoStage (Variables|Default|GetPlayerPawn)) "NewEnumerator3")
    (CallFunction|DemolishNucleus (Variables|Default|GetEyes_180510_3_Lens_Nucleus_03) (Variables|Default|GetEyes_Lens_Nucleus_03_DM))))

(event OnComponentBeginOverlap(Eyes_180510_3_Lens_Nucleus_04)
  (params (OverlappedComponent :type Primitive%20Component%20Object%20Reference) (OtherActor :type Actor%20Object%20Reference) (OtherComp :type Primitive%20Component%20Object%20Reference) (OtherBodyIndex :type Integer) (bFromSweep :type Boolean) (SweepResult :type Hit%20Result%20Structure%20%28by%20ref%29))
  ;[1 1 1] Nucleus Remove
  (Utilities|Casting|CastToBP_Hand_Phaco OtherActor)
  (Utilities|FlowControl|Delay 0.5)
  (if (Utilities|Enum|Equal(Enum) (Variables|/Game/1_Blueprint/Player/BP_OptitrackPlayer.BP_OptitrackPlayer_C|GetPhacoStage (Variables|Default|GetPlayerPawn)) "NewEnumerator3")
    (CallFunction|DemolishNucleus (Variables|Default|GetEyes_180510_3_Lens_Nucleus_04) (Variables|Default|GetEyes_Lens_Nucleus_04_DM))))

(event OnComponentEndOverlap(Eye_Lens)
  (params (OverlappedComponent :type Primitive%20Component%20Object%20Reference) (OtherActor :type Actor%20Object%20Reference) (OtherComp :type Primitive%20Component%20Object%20Reference) (OtherBodyIndex :type Integer))
  ;[1 1 1] Lens Region Event
  (Utilities|Casting|CastToBP_Hand_Phaco OtherActor)
  (Variables|Default|SetEnteredLensRegion true))

(event Custom|OnComponentBeginOverlap_이벤트_1
  (params (OverlappedComponent :type Primitive%20Component%20Object%20Reference) (OtherActor :type Actor%20Object%20Reference) (OtherComp :type Primitive%20Component%20Object%20Reference) (OtherBodyIndex :type Integer) (bFromSweep :type Boolean) (SweepResult :type Hit%20Result%20Structure%20%28by%20ref%29))
  ;[1 1 1] Setup Collision Event
  (if (Utilities|Enum|Equal(Enum) (Variables|Default|GetPhacoStep) "NewEnumerator12")
    (Utilities|Casting|CastToBP_MotionController OtherActor)
    (CallFunction|BeginOverlap OverlappedComponent OtherActor OtherComp OtherBodyIndex bFromSweep SweepResult false)
    (Collision|SetCollisionEnabled OverlappedComponent "NoCollision")
    (if (Utilities|Enum|Equal(Enum) (Utilities|GetObjectName OverlappedComponent) "Box22")
      (bind _checked (CallFunction|CheckBoxArray (Variables|Default|GetVerticalBoxArray)))
      (if _checked
        (Utilities|FlowControl|Delay 1.0)
        (Transformation|AddRelativeLocation (Variables|Default|GetPickBoxVertical) "-100000.000000, 0, 0" false false)))))

(event Custom|SetupCollsionEvent
  ;[1 1 1] Setup Collision Event
  (Utilities|FlowControl|Sequence
    (:then_0
      (Utilities|Array|Add (Variables|Default|GetHorizonBoxArray) (Variables|Default|GetBox2))
      (Utilities|Array|Add (Variables|Default|GetHorizonBoxArray) (Variables|Default|GetBox3))
      (Utilities|Array|Add (Variables|Default|GetHorizonBoxArray) (Variables|Default|GetBox4))
      (Utilities|Array|Add (Variables|Default|GetHorizonBoxArray) (Variables|Default|GetBox5))
      (Utilities|Array|Add (Variables|Default|GetHorizonBoxArray) (Variables|Default|GetBox6))
      (Utilities|Array|Add (Variables|Default|GetHorizonBoxArray) (Variables|Default|GetBox7))
      (Utilities|Array|Add (Variables|Default|GetHorizonBoxArray) (Variables|Default|GetBox8))
      (Utilities|Array|Add (Variables|Default|GetHorizonBoxArray) (Variables|Default|GetBox9))
      (Utilities|Array|Add (Variables|Default|GetHorizonBoxArray) (Variables|Default|GetBox10)))
    (:then_1
      (Utilities|Array|Add (Variables|Default|GetVerticalBoxArray) (Variables|Default|GetBox14))
      (Utilities|Array|Add (Variables|Default|GetVerticalBoxArray) (Variables|Default|GetBox15))
      (Utilities|Array|Add (Variables|Default|GetVerticalBoxArray) (Variables|Default|GetBox16))
      (Utilities|Array|Add (Variables|Default|GetVerticalBoxArray) (Variables|Default|GetBox17))
      (Utilities|Array|Add (Variables|Default|GetVerticalBoxArray) (Variables|Default|GetBox18))
      (Utilities|Array|Add (Variables|Default|GetVerticalBoxArray) (Variables|Default|GetBox19))
      (Utilities|Array|Add (Variables|Default|GetVerticalBoxArray) (Variables|Default|GetBox20))
      (Utilities|Array|Add (Variables|Default|GetVerticalBoxArray) (Variables|Default|GetBox21))
      (Utilities|Array|Add (Variables|Default|GetVerticalBoxArray) (Variables|Default|GetBox22)))
    (:then_2
      (for _array_element (Variables|Default|GetHorizonBoxArray)
        (Collision|AssignOnComponentBeginOverlap _array_element (delegate Custom|OnComponentBeginOverlap_이벤트_0))))
    (:then_3
      (for _array_element_2 (Variables|Default|GetVerticalBoxArray)
        (Collision|AssignOnComponentBeginOverlap _array_element_2 (delegate Custom|OnComponentBeginOverlap_이벤트_1))))
    (:then_4
      (Collision|AssignOnComponentBeginOverlap (Variables|Default|GetBox) (delegate Custom|OnComponentBeginOverlap_이벤트_2)))))

(event Custom|InhalatNucleus
  (params (ApartNucleus :type Destructible%20Component%20Object%20Reference))
  ;[1 1 1] Inhalat Nucleus Event
  (if (Utilities|Enum|Equal(Enum) (Variables|Default|GetPhacoStep) "NewEnumerator15")
    (bind _scale (Timeline|타임라인_3 PlayFromStart)
      (:Update
        (Transformation|SetRelativeScale3D ApartNucleus (Math|Vector|MakeVector _scale _scale _scale)))
      (:Finished
        (bind _returnvalue (Utilities|Array|Add (Variables|Default|GetApartNucleusArray) ApartNucleus))
        (if (not (== _returnvalue 3))
          (CallFunction|TickNucleusEffect))))))

(event Custom|AnimateCracking
  ;[1 1 1] AnimateCracking Event
  (bind _asui_image_base (Utilities|Casting|CastToUI_ImageBase (UserInterface|GetUserWidgetObject (Variables|Default|GetCrossArrow))))
  (Default|PlayTotalFadeEffect _asui_image_base 1.0)
  (Rendering|SetVisibility (Variables|Default|GetCrossArrow) true false)
  (Utilities|FlowControl|Delay 1.0)
  (bind _dist (Timeline|타임라인_1 PlayFromStart)
    (:Update
      (Utilities|FlowControl|Sequence
        (:then_0
          (Transformation|SetRelativeLocation (Variables|Default|GetEyes_180510_3_Lens_Nucleus_01) (* (Math|Vector|MakeVector -1.0 0.0 1.0) _dist) false false))
        (:then_1
          (Transformation|SetRelativeLocation (Variables|Default|GetEyes_180510_3_Lens_Nucleus_02) (* (Math|Vector|MakeVector 1.0 0.0 -1.0) _dist) false false))
        (:then_2
          (Transformation|SetRelativeLocation (Variables|Default|GetEyes_180510_3_Lens_Nucleus_03) (* (Math|Vector|MakeVector 1.0 0.0 1.0) _dist) false false))
        (:then_3
          (Transformation|SetRelativeLocation (Variables|Default|GetEyes_180510_3_Lens_Nucleus_04) (* (Math|Vector|MakeVector -1.0 0.0 -1.0) _dist) false false))))
    (:Finished
      (Utilities|FlowControl|Delay 0.1)
      (CallFunction|SetCourseComplete))))

(event Custom|AnimateCurvedArrow
  ;[1 1 1] AnimateCurvedArrow Event
  (Utilities|FlowControl|Delay 1.0)
  (bind _asui_image_base (Utilities|Casting|CastToUI_ImageBase (UserInterface|GetUserWidgetObject (Variables|Default|GetCurvedArrow))))
  (Default|PlayTotalFadeEffect _asui_image_base 1.0)
  (Rendering|SetVisibility (Variables|Default|GetCurvedArrow) true false)
  (bind _curvedarrowangle (Timeline|타임라인_0 PlayFromStart)
    (:Update
      (Transformation|SetRelativeLocationAndRotation (Variables|Default|GetCurvedArrow) (+ (Math|Vector|RotateVectorAroundAxis "0.000000,0.000000,3.000000" _curvedarrowangle "0.000000,1.000000,0.000000") "0,8.000000, 0") (Math|Rotator|MakeRotator (+ (* _curvedarrowangle -1.0) -45.0) 0.0 9e+01) false false))))

(event Custom|DemolishNucleus
  (params (NucleusObj :type Primitive%20Component%20Object%20Reference) (DestructableObj :type Destructible%20Component%20Object%20Reference))
  ;[1 1 1] Demolish Nucleus Event
  (if (Utilities|Enum|Equal(Enum) (Variables|Default|GetPhacoStep) "NewEnumerator15")
    (Components|DestroyComponent NucleusObj)
    (Class|DestructibleComponent|ApplyRadiusDamage DestructableObj 1e+01 (Transformation|GetWorldLocation DestructableObj) 5.0 5.0 false)
    (CallFunction|InhalatNucleus DestructableObj)))

(event Custom|OnComponentBeginOverlap_이벤트_2
  (params (OverlappedComponent :type Primitive%20Component%20Object%20Reference) (OtherActor :type Actor%20Object%20Reference) (OtherComp :type Primitive%20Component%20Object%20Reference) (OtherBodyIndex :type Integer) (bFromSweep :type Boolean) (SweepResult :type Hit%20Result%20Structure%20%28by%20ref%29))
  ;[1 1 1] Setup Collision Event
  (if (Utilities|Enum|Equal(Enum) (Variables|Default|GetPhacoStep) "NewEnumerator12")
    (Utilities|Casting|CastToBP_MotionController OtherActor)
    (CallFunction|BeginOverlap OverlappedComponent OtherActor OtherComp OtherBodyIndex bFromSweep SweepResult false)
    (Collision|SetCollisionEnabled OverlappedComponent "NoCollision")))

(event Custom|AnimateNucleusEffect
  (params (EffectObj :type Static%20Mesh%20Component%20Object%20Reference))
  (bind _nucleusfocusingmaterial (Variables|Default|GetNucleusFocusingMaterial))
  (bind (_value _returnvalue) (Utilities|Map|Find _nucleusfocusingmaterial EffectObj))
  ;[1 1 1] Animate Nucleus Bloom Effect
  (if _returnvalue
    (bind _angle (Timeline|타임라인_2 PlayFromStart)
      (:Update
        (Rendering|Material|SetScalarParameterValue _value "Weight" (+ (* (Math|Trig|Cos(Degrees) _angle) 0.5) 0.5) :!class /Script/Engine.MaterialInstanceDynamic))
      (:Finished
        (Utilities|FlowControl|Delay 0.5)
        (bind _asstatic_mesh_component (Utilities|Casting|CastToStaticMeshComponent (Transformation|GetAttachParent EffectObj)))
        (Collision|SetCollisionEnabled _asstatic_mesh_component "QueryAndPhysics")
        (Components|DestroyComponent EffectObj)))))

(event Custom|OnComponentBeginOverlap_이벤트_0
  (params (OverlappedComponent :type Primitive%20Component%20Object%20Reference) (OtherActor :type Actor%20Object%20Reference) (OtherComp :type Primitive%20Component%20Object%20Reference) (OtherBodyIndex :type Integer) (bFromSweep :type Boolean) (SweepResult :type Hit%20Result%20Structure%20%28by%20ref%29))
  ;[1 1 1] Setup Collision Event
  (if (Utilities|Enum|Equal(Enum) (Variables|Default|GetPhacoStep) "NewEnumerator20")
    (Utilities|Casting|CastToBP_MotionController OtherActor)
    (CallFunction|BeginOverlap OverlappedComponent OtherActor OtherComp OtherBodyIndex bFromSweep SweepResult true)
    (Collision|SetCollisionEnabled OverlappedComponent "NoCollision")
    (if (Utilities|Enum|Equal(Enum) (Utilities|GetObjectName OverlappedComponent) "Box10")
      (bind _checked (CallFunction|CheckBoxArray (Variables|Default|GetHorizonBoxArray)))
      (if _checked
        (Utilities|FlowControl|Delay 1.0)
        (Transformation|AddRelativeLocation (Variables|Default|GetPickBoxHorizon) "100000.000000, 0, 0" false false)))))

(event EventBeginPlay
  ;[1 1 1] Begin Event
  (CallFunction|SetPlayer)
  (CallFunction|SetupCollsionEvent)
  (CallFunction|SetProceduralMeshes)
  (CallFunction|SetNucleusEffect))

(event EventTick
  (params (DeltaSeconds :type Float%20%28single-precision%29))
  ;[1 1 1] Tick Event
  (switch Utilities|FlowControl|Switch|SwitchonE_TraningCourse (Variables|Default|GetPhacoStep)
    (:NewEnumerator13
      (if (and (Utilities|Enum|Equal(Enum) (Variables|/Game/1_Blueprint/Player/BP_OptitrackPlayer.BP_OptitrackPlayer_C|GetPhacoStage (Variables|Default|GetPlayerPawn)) "NewEnumerator1") (Variables|Default|GetEnteredVerticalRegion))
        (CallFunction|CalculateCurrentAngle)))
    (:NewEnumerator15
      (if (== (Utilities|Array|Length (Variables|Default|GetApartNucleusArray)) 4)
        (if (Utilities|Enum|Equal(Enum) (Variables|/Game/1_Blueprint/Player/BP_OptitrackPlayer.BP_OptitrackPlayer_C|GetPhacoStage (Variables|Default|GetPlayerPawn)) "NewEnumerator2")
          (CallFunction|SetCourseComplete))))))

(fn ConstructionScript)

(fn BeginOverlap
  (params (OverlappedComponent :type Primitive%20Component%20Object%20Reference) (OtherActor :type Actor%20Object%20Reference) (OtherComp :type Primitive%20Component%20Object%20Reference) (OtherBodyIndex :type Integer) (FromSweep :type Boolean) (SweepResult :type Hit%20Result%20Structure) (IsHorizontal :type Boolean))
  (bind _asbox_collision (Utilities|Casting|CastToBoxComponent OverlappedComponent))
  (LocalVariables|SetCurrBox _asbox_collision)
  (Utilities|Casting|CastToBP_MotionController OtherActor)
  (if (Utilities|Enum|Equal(Enum) (Variables|/Game/1_Blueprint/Player/BP_OptitrackPlayer.BP_OptitrackPlayer_C|GetPhacoStage (Variables|Default|GetPlayerPawn)) "NewEnumerator3")
    (if (> (Class|SceneComponent|GetNumChildrenComponents (LocalVariables|GetCurrBox)) 0)
      (bind _asstatic_mesh_component (Utilities|Casting|CastToStaticMeshComponent (Components|GetChildComponent (LocalVariables|GetCurrBox) 0)))
      (Utilities|FlowControl|Sequence
        (:then_0
          (if IsHorizontal
            (bind _outotherhalfprocmesh (Class|KismetProceduralMeshLibrary|SliceProceduralMesh (Variables|Default|GetLens_Nucleus_Horizon) (Transformation|GetWorldLocation _asstatic_mesh_component) (Math|Vector|GetUpVector _asstatic_mesh_component) true "CreateNewSectionForCap"))
            (Components|DestroyComponent _outotherhalfprocmesh)
            (else
              (bind _outotherhalfprocmesh_2 (Class|KismetProceduralMeshLibrary|SliceProceduralMesh (Variables|Default|GetLens_Nucleus_Vertical) (Transformation|GetWorldLocation _asstatic_mesh_component) (Math|Vector|GetUpVector _asstatic_mesh_component) true "CreateNewSectionForCap"))
              (Components|DestroyComponent _outotherhalfprocmesh_2))))
        (:then_1
          (Collision|SetCollisionEnabled (LocalVariables|GetCurrBox) "NoCollision")))
      (elif (== (LocalVariables|GetCurrBox) (Variables|Default|GetBox))
        (Rendering|SetVisibility (Variables|Default|GetEyes_180510_3_Lens_Nucleus_Center) false true)))))

(fn SetProceduralMeshes
  (Class|KismetProceduralMeshLibrary|CopyProceduralMeshfromStaticMeshComponent (Variables|Default|GetEyes_180510_3_Lens_Nucleus_Horizon) 0 (Variables|Default|GetLens_Nucleus_Horizon) true)
  (Class|KismetProceduralMeshLibrary|CopyProceduralMeshfromStaticMeshComponent (Variables|Default|GetEyes_180510_3_Lens_Nucleus_Vertical) 0 (Variables|Default|GetLens_Nucleus_Vertical) true))

(fn PreparePhacoStep
  (params (Course :type E_TraningCourse%20Enum :default "NewEnumerator4"))
  (Variables|Default|SetPhacoStep Course)
  (switch Utilities|FlowControl|Switch|SwitchonE_TraningCourse (Variables|Default|GetPhacoStep)
    (:NewEnumerator12
      ;[1 1 1] Vertical Phaco sculpting
      (Transformation|AttachComponentToComponent (Variables|Default|GetArrow) (Variables|Default|GetArrowVertical) "None" "KeepRelative" "KeepRelative" "KeepRelative" true)
      (Rendering|SetVisibility (Variables|Default|GetArrowVertical) true true)
      (Utilities|FlowControl|Sequence
        (:then_0
          (bind _asui_image_base (Utilities|Casting|CastToUI_ImageBase (UserInterface|GetUserWidgetObject (Variables|Default|GetSculptingAreaVertical))))
          (Default|PlayTotalFadeEffect _asui_image_base 0.5))
        (:then_1
          (bind _asui_image_base_2 (Utilities|Casting|CastToUI_ImageBase (UserInterface|GetUserWidgetObject (Variables|Default|GetArrow))))
          (Default|PlayTotalFadeEffect _asui_image_base_2 0.5))))
    (:NewEnumerator13
      ;[1 1 1] Rotating the necleus
      (CallFunction|AnimateCurvedArrow))
    (:NewEnumerator20
      ;[1 1 1] Horizon Phaco sculpting
      (Transformation|AttachComponentToComponent (Variables|Default|GetArrow) (Variables|Default|GetArrowHorizon) "None" "KeepRelative" "KeepRelative" "KeepRelative" true)
      (Rendering|SetVisibility (Variables|Default|GetArrowHorizon) true true)
      (Utilities|FlowControl|Sequence
        (:then_0
          (bind _asui_image_base_3 (Utilities|Casting|CastToUI_ImageBase (UserInterface|GetUserWidgetObject (Variables|Default|GetSculptingAreaHorizon))))
          (Default|PlayTotalFadeEffect _asui_image_base_3 0.5))
        (:then_1
          (bind _asui_image_base_4 (Utilities|Casting|CastToUI_ImageBase (UserInterface|GetUserWidgetObject (Variables|Default|GetArrow))))
          (Default|PlayTotalFadeEffect _asui_image_base_4 0.5))))
    (:NewEnumerator14
      ;[1 1 1] Cracking
      (CallFunction|AnimateCracking))
    (:NewEnumerator15
      ;[1 1 1] Removing quadrants of necleus
      (Rendering|SetVisibility (Variables|Default|GetEyes_180510_3_Lens_Nucleus_01) false false)
      (Rendering|SetVisibility (Variables|Default|GetEyes_180510_3_Lens_Nucleus_02) false false)
      (Rendering|SetVisibility (Variables|Default|GetEyes_180510_3_Lens_Nucleus_03) false false)
      (Rendering|SetVisibility (Variables|Default|GetEyes_180510_3_Lens_Nucleus_04) false false)
      (CallFunction|TickNucleusEffect))))

(fn CheckBoxArray
  (params (BoxArray :type Array%20of%20Box%20Component%20Object%20References))
  (for _index (range 0 (- (Utilities|Array|Length BoxArray) 2))
    (if (Utilities|Enum|Equal(Enum) (Collision|GetCollisionEnabled (Utilities|Array|Get(acopy) BoxArray _index)) "QueryOnly")
      (return true)))
  (return true))

(fn GetPickBox
  (params (Vertical :type Boolean))
  (if Vertical
    (bind _asbp_pick_obj_base (Utilities|Casting|CastToBP_PickObjBase (Variables|/Script/Engine.ChildActorComponent|GetChildActor (Variables|Default|GetPickBoxVertical)))
      (:then
        (return _asbp_pick_obj_base))
      (:CastFailed
        (return 0)))
    (else
      (bind _asbp_pick_obj_base_2 (Utilities|Casting|CastToBP_PickObjBase (Variables|/Script/Engine.ChildActorComponent|GetChildActor (Variables|Default|GetPickBoxHorizon)))
        (:then
          (return _asbp_pick_obj_base_2))
        (:CastFailed
          (return 0))))))

(fn CalculateCurrentAngle
  (bind _vector0 (Variables|Default|GetVector0))
  (LocalVariables|Setdot (Math|Vector|DotProduct (Math|Vector|Normalize (- (Transformation|GetWorldLocation (Variables|/Game/1_Blueprint/MotionVR/BP_HandBase.BP_HandBase_C|GetPoint (Variables|Default|GetHand_Phaco))) (Transformation|GetWorldLocation (Variables|Default|GetCenter)))) _vector0))
  (LocalVariables|Setcross (Math|Vector|Normalize (Math|Vector|CrossProduct (Math|Vector|Normalize (- (Transformation|GetWorldLocation (Variables|/Game/1_Blueprint/MotionVR/BP_HandBase.BP_HandBase_C|GetPoint (Variables|Default|GetHand_Phaco))) (Transformation|GetWorldLocation (Variables|Default|GetCenter)))) _vector0)))
  (Utilities|FlowControl|Sequence
    (:then_0
      (LocalVariables|Setangle (* (Class|KismetMathLibrary|DegAcos (LocalVariables|Getdot)) (LocalVariables|Getdirection_const))))
    (:then_1
      (Transformation|AddLocalRotation (Variables|Default|GetScene) (Math|Rotator|MakeRotator 0.0 (LocalVariables|Getangle) 0.0) false false)
      (if (Math|Float|NearlyEqual(Float) (.Pitch (Math|Rotator|BreakRotator (Variables|/Script/Engine.SceneComponent|GetRelativeRotation (Variables|Default|GetScene)))) -45.0 5.0)
        (Variables|Default|SetHand_Phaco 0)
        (Transformation|SetRelativeRotation (Variables|Default|GetScene) "-45.000000, 0, 0" false false)
        (CallFunction|SetCourseComplete)))))

(fn CalculateVector
  (return (Math|Vector|Normalize (- (Transformation|GetWorldLocation (Variables|/Game/1_Blueprint/MotionVR/BP_HandBase.BP_HandBase_C|GetPoint (Variables|Default|GetHand_Phaco))) (Transformation|GetWorldLocation (Variables|Default|GetCenter))))))

(fn TickNucleusEffect
  (switch int (Utilities|Array|Length (Variables|Default|GetApartNucleusArray))
    (:0
      (Utilities|IsValid (Variables|Default|GetEyes_Lens_Nucleus_01_Edge)
        (:Is%20Valid
          (CallFunction|AnimateNucleusEffect (Variables|Default|GetEyes_Lens_Nucleus_01_Edge)))))
    (:1
      (Utilities|IsValid (Variables|Default|GetEyes_Lens_Nucleus_02_Edge)
        (:Is%20Valid
          (CallFunction|AnimateNucleusEffect (Variables|Default|GetEyes_Lens_Nucleus_02_Edge)))))
    (:2
      (Utilities|IsValid (Variables|Default|GetEyes_Lens_Nucleus_03_Edge)
        (:Is%20Valid
          (CallFunction|AnimateNucleusEffect (Variables|Default|GetEyes_Lens_Nucleus_03_Edge)))))
    (:3
      (Utilities|IsValid (Variables|Default|GetEyes_Lens_Nucleus_04_Edge)
        (:Is%20Valid
          (CallFunction|AnimateNucleusEffect (Variables|Default|GetEyes_Lens_Nucleus_04_Edge)))))))

(fn SetNucleusEffect
  (bind _eyes_lens_nucleus_01_edge (Variables|Default|GetEyes_Lens_Nucleus_01_Edge))
  (bind _eyes_lens_nucleus_02_edge (Variables|Default|GetEyes_Lens_Nucleus_02_Edge))
  (bind _eyes_lens_nucleus_03_edge (Variables|Default|GetEyes_Lens_Nucleus_03_Edge))
  (bind _eyes_lens_nucleus_04_edge (Variables|Default|GetEyes_Lens_Nucleus_04_Edge))
  (Utilities|FlowControl|Sequence
    (:then_0
      (bind _returnvalue (Rendering|Material|CreateDynamicMaterialInstance _eyes_lens_nucleus_01_edge 0 (Rendering|Material|GetMaterial _eyes_lens_nucleus_01_edge 0) :!class /Script/Engine.PrimitiveComponent))
      (Utilities|Map|Add (Variables|Default|GetNucleusFocusingMaterial) _eyes_lens_nucleus_01_edge _returnvalue)
      (Collision|SetCollisionEnabled (Variables|Default|GetEyes_180510_3_Lens_Nucleus_01) "NoCollision"))
    (:then_1
      (bind _returnvalue_2 (Rendering|Material|CreateDynamicMaterialInstance _eyes_lens_nucleus_02_edge 0 (Rendering|Material|GetMaterial _eyes_lens_nucleus_02_edge 0) :!class /Script/Engine.PrimitiveComponent))
      (Utilities|Map|Add (Variables|Default|GetNucleusFocusingMaterial) _eyes_lens_nucleus_02_edge _returnvalue_2)
      (Collision|SetCollisionEnabled (Variables|Default|GetEyes_180510_3_Lens_Nucleus_02) "NoCollision"))
    (:then_2
      (bind _returnvalue_3 (Rendering|Material|CreateDynamicMaterialInstance _eyes_lens_nucleus_03_edge 0 (Rendering|Material|GetMaterial _eyes_lens_nucleus_03_edge 0) :!class /Script/Engine.PrimitiveComponent))
      (Utilities|Map|Add (Variables|Default|GetNucleusFocusingMaterial) _eyes_lens_nucleus_03_edge _returnvalue_3)
      (Collision|SetCollisionEnabled (Variables|Default|GetEyes_180510_3_Lens_Nucleus_03) "NoCollision"))
    (:then_3
      (bind _returnvalue_4 (Rendering|Material|CreateDynamicMaterialInstance _eyes_lens_nucleus_04_edge 0 (Rendering|Material|GetMaterial _eyes_lens_nucleus_04_edge 0) :!class /Script/Engine.PrimitiveComponent))
      (Utilities|Map|Add (Variables|Default|GetNucleusFocusingMaterial) _eyes_lens_nucleus_04_edge _returnvalue_4)
      (Collision|SetCollisionEnabled (Variables|Default|GetEyes_180510_3_Lens_Nucleus_04) "NoCollision"))))

(fn SetPlayer
  (bind _asbp_optitrack_player (Utilities|Casting|CastToBP_OptitrackPlayer (Game|Player|GetPlayerPawn 0)))
  (Variables|Default|SetPlayerPawn _asbp_optitrack_player))

(fn SetCourseComplete
  (Default|CatchCourseCompleted (Variables|Default|GetPlayerPawn))
  (Variables|Default|SetPhacoStep "NewEnumerator4"))